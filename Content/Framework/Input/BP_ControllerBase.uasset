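; Base player controller that opens the character creation widget on BeginPlay and handles player unit spawning, possession and camera zoom.
; The zoom input sets a clamped target arm length, which Tick interpolates onto the unit's spring arm.
; Camera world pitch follows a float curve sampled by normalized arm length, with yaw and roll fixed at zero.
; Spawning ignores the UnitType argument and uses DA_TheGuy; key 1 prints Strength for debugging.
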(event Input|EnhancedActionEvents|EnhancedInputActionIA_ZoomScroll
  (params (ActionValue :type Float%20%28double-precision%29) (ElapsedSeconds :type Float%20%28double-precision%29) (TriggeredSeconds :type Float%20%28double-precision%29) (InputAction :type Input%20Action%20Object%20Reference :default "/Game/Framework/Input/InputAction/IA_ZoomScroll.IA_ZoomScroll"))
  ;[0.15 0.15 0.15 0.5] Scroll
  (CallFunction|Scroll ActionValue))

(event EventBeginPlay
  (CallFunction|Initialize))

(event EventTick
  (params (DeltaSeconds :type Float%20%28single-precision%29))
  ;[0.15 0.15 0.15 0.5] Scroll
  (CallFunction|UpdateScroll DeltaSeconds))

(event Input|KeyboardEvents|1
  (params (Key :type Key%20Structure :default "None"))
  (:Pressed
    (Development|PrintString (Utilities|String|ToString(Float) (Class|AttributeComponent|GetAttribute (Variables|/Script/Project_A.UnitBase|GetAttributeComponent (Variables|Default|GetUnitRef)) "Strength")))))

(fn ConstructionScript)

(fn Initialize
  (bind _returnvalue (UserInterface|CreateWidget "/Game/Framework/UI/CharacterCreate.CharacterCreate_C"))
  (Default|SetControllerRef _returnvalue self)
  (UserInterface|Viewport|AddtoViewport _returnvalue 0))

(fn Scroll
  (params (ActionValue :type Float%20%28double-precision%29))
  (Utilities|IsValid (Variables|Default|GetPlayerUnit)
    (:Is%20Valid
      (Variables|Default|SetTargetArmLength (Math|Float|Clamp(Float) (+ (* ActionValue (Variables|Default|GetScrollStrength) -1.0) (Variables|Default|GetTargetArmLength)) (Variables|Default|GetMinScroll) (Variables|Default|GetMaxScroll))))))

(fn UpdateScroll
  (params (DeltaTime :type Float%20%28double-precision%29))
  (Utilities|IsValid (Variables|Default|GetPlayerUnit)
    (:Is%20Valid
      (bind _output_get (Variables|/Script/Engine.SpringArmComponent|SetTargetArmLength (Variables|/Script/Project_A.PlayerUnit|GetSpringArm (Variables|Default|GetPlayerUnit)) (Math|Interpolation|FInterpTo (Utilities|GetSpringArmLength) (Variables|Default|GetTargetArmLength) DeltaTime 1.0)))
      (CallFunction|RotateCameraAlongCurve _output_get))))

(fn RotateCameraAlongCurve
  (params (Value :type Float%20%28double-precision%29))
  ;[0.15 0.15 0.15 0.5] Takes current arm length, normalizes it between min/max and finds the corresponding rotation on CameraCurve
  (Transformation|SetWorldRotation (Variables|/Script/Project_A.PlayerUnit|GetCamera (Variables|Default|GetPlayerUnit)) (Math|Rotator|MakeRotator 0.0 (Math|Curves|GetFloatValue (Variables|Default|GetCameraCurve) (Math|Float|NormalizetoRange Value (Variables|Default|GetMinScroll) (Variables|Default|GetMaxScroll))) 0.0) false false))

(fn SpawnPlayerUnit
  (params (UnitType :type %20Object%20Reference))
  (bind _returnvalue (Class|UnitSpawner|SpawnPlayerUnit (Subsystems|GetUnitSpawner) "/Game/DataAsset/PlayerCharacters/DA_TheGuy.DA_TheGuy"))
  (bind _output_get (Variables|Default|SetUnitRef _returnvalue))
  (Class|ControllerBase|PossessPlayerUnit _output_get))